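; A swinging door that the first-person player can open and close through an OpenDoor event.
; A timeline rotates the door up to 90 degrees, with the swing side picked by a dot product of player position and door forward vector.
; Calling the event again reverses the timeline, and the closed flag resets when that finishes.
; A box trigger shows a billboard while the player overlaps it.
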(event OnComponentBeginOverlap(Box)
  (params (OverlappedComponent :type Primitive%20Component%20Object%20Reference) (OtherActor :type Actor%20Object%20Reference) (OtherComp :type Primitive%20Component%20Object%20Reference) (OtherBodyIndex :type Integer) (bFromSweep :type Boolean) (SweepResult :type Hit%20Result%20Structure%20%28by%20ref%29))
  (Utilities|Casting|CastToFirstPersonCharacter OtherActor)
  (Rendering|SetVisibility (Variables|Default|GetBillboard) true false))

(event OnComponentEndOverlap(Box)
  (params (OverlappedComponent :type Primitive%20Component%20Object%20Reference) (OtherActor :type Actor%20Object%20Reference) (OtherComp :type Primitive%20Component%20Object%20Reference) (OtherBodyIndex :type Integer))
  (Utilities|Casting|CastToFirstPersonCharacter OtherActor)
  (Rendering|SetVisibility (Variables|Default|GetBillboard) false false))

(event Custom|OpenDoor
  (if (Variables|Default|GetIsDoorClosed?)
    (Variables|Default|SetIsDoorClosed? false)
    (Variables|Default|SetDotProduct (Math|Vector|DotProduct (Math|Vector|Normalize (- (Transformation|GetWorldLocation (Variables|Default|GetScene)) (Transformation|GetActorLocation (Variables|Default|GetPlayerREF)))) (Math|Vector|GetForwardVector (Variables|Default|GetScene))))
    (bind (_direction _track_1) (Timeline|Open/Close%20Door PlayFromStart)
      (:Update
        (Transformation|SetRelativeRotation (Variables|Default|GetDoor) (Math|Rotator|MakeRotator 0.0 0.0 (Math|Float|Lerp 0.0 (Math|Float|SelectFloat 9e+01 -9e+01 (>= (Variables|Default|GetDotProduct) 0.0)) _track_1)) false false))
      (:Finished
        (switch Utilities|FlowControl|Switch|SwitchonETimelineDirection _direction
          (:Backward
            (Variables|Default|SetIsDoorClosed? true)))))
    (else
      (Timeline|Open/Close%20Door ReverseFromEnd))))

(event EventBeginPlay
  (bind _asfirst_person_character (Utilities|Casting|CastToFirstPersonCharacter (Game|GetPlayerCharacter 0)))
  (Variables|Default|SetPlayerREF _asfirst_person_character))

(fn ConstructionScript)